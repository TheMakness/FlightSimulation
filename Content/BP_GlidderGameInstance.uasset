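; Game instance for the Glidder game that holds playtest session data and saves it to disk as JSON.
; On Shutdown it records the total test time from real-time seconds, then calls SaveData.
; SaveData copies the GameData struct into a new GameData object, converts it to JSON and writes it to the project's Content/Data folder.
; The filename combines tester name with UTC day and month.
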(event `SaveData`
  (bind (_returnvalue_year _returnvalue_month _returnvalue_day) (`KismetMathLibrary.BreakDateTime` (`KismetMathLibrary.GetDate` (`KismetMathLibrary.UtcNow`))))
  (bind _returnvalue (`|GenericCreateObject` "/Game/GameData.GameData_C"))
  (set `/Game/GameData.Data` (`self.GameData`) _returnvalue)
  (`JsonBlueprintFunctionLibrary.ToFile` (`JsonSerializationBlueprintFunctionLibrary.ObjectToJson` _returnvalue) (make `FilePath` (`KismetStringLibrary.Concat_StrStr` (`KismetSystemLibrary.GetProjectContentDirectory`) (`KismetStringLibrary.Concat_StrStr` "Data/" (`.TesterName_2_6B7C5B0742A62A163F0854B35C81E100` (break `/Game/SessionData` (`self.GameData`))) "_" (`KismetStringLibrary.Conv_IntToString` _returnvalue_day) "-" (`KismetStringLibrary.Conv_IntToString` _returnvalue_month) ".json")))))

(event `self.ReceiveShutdown`
  (setmembers `/Game/SessionData` :`StructRef` (`self.GameData`) :`TotalTestTime` (`GameplayStatics.GetRealTimeSeconds`))
  (`self.SaveData`))