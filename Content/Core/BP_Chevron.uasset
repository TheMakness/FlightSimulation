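; BP_Chevron is a track marker that shows only when it lies ahead of the player within the current checkpoint segment.
; On its first Tick it caches the BP_CheckpointManager.
; Every Tick it compares its spline position with the current and next checkpoints' SplineAlpha and player pawn 0's position, using small margins, then toggles its hidden-in-game state.
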(event `self.ReceiveBeginPlay`)

(event `self.ReceiveTick`
  (params (DeltaSeconds :type "Float (single-precision)"))
  (bind _checkpointmanager (`self.CheckpointManager`))
  (bind _time (`self.GetTimeAtLocationAlongSpline` (`self.K2_GetActorLocation`)))
  (`|ExecutionSequence`
    (:`then_0`
      (`/Engine/EditorBlueprintResources/StandardMacros.DoOnce` false
        (:`Completed`
          (bind _outactors (`GameplayStatics.GetAllActorsOfClass` "/Game/Core/Glider/BP_CheckpointManager.BP_CheckpointManager_C"))
          (set `self.CheckpointManager` (`|GetArrayItem` _outactors)))))
    (:`then_1`
      (if (and (> _time (`/Game/Core/Glider/BP_Checkpoint.SplineAlpha` (`/Game/Core/Glider/BP_CheckpointManager.CurrentCheckpoint` _checkpointmanager))) (< _time (+ (`/Game/Core/Glider/BP_Checkpoint.SplineAlpha` (`/Game/Core/Glider/BP_CheckpointManager.NextCheckpoint` _checkpointmanager)) 0.005)) (> _time (+ (`self.GetTimeAtLocationAlongSpline` (`self.K2_GetActorLocation` (`GameplayStatics.GetPlayerPawn` 0))) 0.0008)))
        (`self.UnHide`)
        (else
          (`self.Hide`))))))

(fn `Hide`
  (`self.SetActorHiddenInGame` true))

(fn `UnHide`
  (`self.SetActorHiddenInGame` false))

(fn `UserConstructionScript`)