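; BP_Checkpoint is a checkpoint actor in a glider game that records when and how accurately the player flies through it.
; On BeginPlay it hides itself and registers its location in the current test's checkpoint list on the game instance; EnableCheckpoint reveals it.
; Box overlap by a Plane records level time, validity and precision from YZ distance to center relative to marker size, then hides it, disables collision and fires Activate.
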(event `self.ReceiveBeginPlay`
  (`self.SetActorHiddenInGame` true)
  (bind _asbp_glidder_game_instance (cast `/Game/BP_GlidderGameInstance` (`GameplayStatics.GetGameInstance`)))
  (cast `/Game/Core/Glider/GliderGameMode` (`GameplayStatics.GetGameMode`))
  (bind (_type _order _time _respawncount _crashcount _checkpointcount _misscheckpointcount _valid _checkpoints) (break `/Game/TestData` (`|GetArrayItem` (`.Tests_21_0D4108294F73791928BF61983873E271` (break `/Game/SessionData` (`/Game/BP_GlidderGameInstance.GameData` _asbp_glidder_game_instance))) (`/Game/BP_GlidderGameInstance.CurrentTestIndex` _asbp_glidder_game_instance))))
  (bind _returnvalue (`KismetArrayLibrary.Array_Add` _checkpoints))
  (setmembers `/Game/CheckpointData` :`StructRef` (`|GetArrayItem` _checkpoints _returnvalue) :`Index` _returnvalue :`Location` (`self.K2_GetActorLocation`)))

(event `self.Box.OnComponentBeginOverlap`
  (params (OverlappedComponent :type "PrimitiveComponent Object Reference") (OtherActor :type "Actor Object Reference") (OtherComp :type "PrimitiveComponent Object Reference") (OtherBodyIndex :type Integer) (bFromSweep :type Boolean) (SweepResult :type "HitResult Structure (by ref)"))
  (cast `/Game/Core/Glider/Plane` OtherActor)
  (`|ExecutionSequence`
    (:`then_0`
      (bind _asbp_glidder_game_instance (cast `/Game/BP_GlidderGameInstance` (`GameplayStatics.GetGameInstance`)))
      (bind _asglider_game_mode (cast `/Game/Core/Glider/GliderGameMode` (`GameplayStatics.GetGameMode`)))
      (setmembers `/Game/CheckpointData` :`StructRef` (`|GetArrayItem` (`.Checkpoints_23_13DDE9CD4772D4199EE11CAB9890E1B1` (break `/Game/TestData` (`|GetArrayItem` (`.Tests_21_0D4108294F73791928BF61983873E271` (break `/Game/SessionData` (`/Game/BP_GlidderGameInstance.GameData` _asbp_glidder_game_instance))) (`/Game/BP_GlidderGameInstance.CurrentTestIndex` _asbp_glidder_game_instance)))) (`self.Index`)) :`ValidationTime` (`/Game/Core/Glider/GliderGameMode.CurrentLevelTimer` _asglider_game_mode) :`Precision` (- 1.0 (/ (`KismetMathLibrary.Distance2D` (`KismetMathLibrary.MakeVector2D` (.y (`self.K2_GetActorLocation`)) (.z (`self.K2_GetActorLocation`))) (`KismetMathLibrary.MakeVector2D` (.y (`self.K2_GetActorLocation` (`GameplayStatics.GetPlayerPawn` 0))) (.z (`self.K2_GetActorLocation` (`GameplayStatics.GetPlayerPawn` 0))))) (* (* (.x (`SceneComponent.RelativeScale3D` (`self.Plane`))) 0.5) 100.0))) :`Valid` true))
    (:`then_1`
      (if (and (`KismetSystemLibrary.IsValid` (`self.Plane`)) (`KismetSystemLibrary.IsValid` (`self.Box`)))
        (`self.SetActorEnableCollision` false)
        (`self.SetActorHiddenInGame` true)))
    (:`then_2`
      (`self.Activate` self (`self.Index`)))))

(fn `EnableCheckpoint`
  (`self.SetActorHiddenInGame` false))

(fn `UserConstructionScript`)