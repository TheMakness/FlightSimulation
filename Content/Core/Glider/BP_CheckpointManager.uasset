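; BP_CheckpointManager sequences the glider checkpoints in a level and advances the game to the next test when the last one is reached.
; On BeginPlay it gathers every BP_Checkpoint, orders them by their Index, binds their activation events and enables the first two.
; Each activation updates the current checkpoint and enables the following two, storing the further one as next.
; Reaching the final checkpoint calls NextTest on BP_GlidderGameInstance.
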(event `self.ReceiveBeginPlay`
  (bind _checkpoints (`self.Checkpoints`))
  (bind _output (`|GetArrayItem` _checkpoints))
  (bind _output_2 (`|GetArrayItem` _checkpoints 1))
  (bind _outactors (`GameplayStatics.GetAllActorsOfClass` "/Game/Core/Glider/BP_Checkpoint.BP_Checkpoint_C"))
  (set `self.Checkpoints` _outactors)
  (for _array_element _outactors
    (`KismetArrayLibrary.Array_Set` (`self.Checkpoints`) (`/Game/Core/Glider/BP_Checkpoint.Index` _array_element) _array_element)
    (add `/Game/Core/Glider/BP_Checkpoint.Activate` _array_element (delegate `OnCheckpointActivate`)))
  (`/Game/Core/Glider/BP_Checkpoint.EnableCheckpoint` _output)
  (set `self.CurrentCheckpoint` _output)
  (`/Game/Core/Glider/BP_Checkpoint.EnableCheckpoint` _output_2)
  (set `self.NextCheckpoint` _output_2))

(event `OnCheckpointActivate`
  (params (Checkpoint :type "/Game/Core/Glider/BP_Checkpoint Object Reference") (Index :type Integer))
  (bind _returnvalue (+ Index 1))
  (bind _returnvalue_2 (+ Index 2))
  (bind _checkpoints (`self.Checkpoints`))
  (bind _output (`|GetArrayItem` (`self.Checkpoints`) (`KismetMathLibrary.SelectInt` _returnvalue_2 Index (`KismetArrayLibrary.Array_IsValidIndex` (`self.Checkpoints`) _returnvalue_2))))
  (set `self.CurrentCheckpoint` Checkpoint)
  (`/Game/Core/Glider/BP_Checkpoint.EnableCheckpoint` (`|GetArrayItem` (`self.Checkpoints`) (`KismetMathLibrary.SelectInt` _returnvalue Index (`KismetArrayLibrary.Array_IsValidIndex` (`self.Checkpoints`) _returnvalue))))
  (`/Game/Core/Glider/BP_Checkpoint.EnableCheckpoint` _output)
  (set `self.NextCheckpoint` _output)
  (if (== (`self.CurrentCheckpoint`) (`|GetArrayItem` _checkpoints (`KismetArrayLibrary.Array_LastIndex` _checkpoints)))
    (bind _asbp_glidder_game_instance (cast `/Game/BP_GlidderGameInstance` (`GameplayStatics.GetGameInstance`)))
    (`/Game/BP_GlidderGameInstance.NextTest` _asbp_glidder_game_instance)))

(fn `UserConstructionScript`)